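; Enemy spawner that fills a fixed-size pool of BP_Enemy actors at random points in a rectangular area around itself.
; A looping timer spawns and stores enemies until SpawnLimit is reached, then stops.
; Deactivated enemies are recycled through their OnEnemyDeactivated dispatcher and reactivated at new random points instead of respawned; bindings clear on EndPlay.
; The construction script sets the spawner's height and draws a debug box based on SpawningArea.
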(event Custom|Loop%20Body
  (bind _returnvalue (Game|SpawnActorfromClass "/Game/Blueprints/BP_Enemy.BP_Enemy_C" (Math|Transform|MakeTransform (CallFunction|GetRandomLocationInsideArea)) "AdjustIfPossibleButAlwaysSpawn" "MultiplyWithRoot" 0 1e+02 1e+01 (Game|GetInstigator)))
  (EventDispatchers|BindEventtoOnEnemyDeactivated _returnvalue (EventDispatchers|CreateEvent :!event Custom|On%20Enemy%20Deactivated))
  (Utilities|Array|SetArrayElem (Variables|Default|GetAll%20Enemies) (Variables|Default|GetSpawn%20Count) _returnvalue)
  (Math|Integer|IncrementInt (Variables|Default|GetSpawn%20Count)
    (:%20%20
      (Development|PrintText (Utilities|Text|FormatText "Spawning... ({SpawnCount})" (Variables|Default|GetSpawn%20Count)))
      (if (>= (Variables|Default|GetSpawn%20Count) (Variables|Properties|GetSpawn%20Limit))
        (Utilities|Time|ClearandInvalidateTimerbyHandle (Variables|Default|GetLoop%20Timer%20Handle))))))

(event Custom|On%20Enemy%20Deactivated
  (params (Enemy :type BP%20Enemy%20Object%20Reference))
  (Default|ActivateActor Enemy (CallFunction|GetRandomLocationInsideArea)))

(event EventBeginPlay
  (bind _returnvalue (Utilities|Time|SetTimerbyEvent (delegate Custom|Loop%20Body) (Variables|Properties|GetSpawn%20Delay) true))
  (Variables|Default|SetLoop%20Timer%20Handle _returnvalue)
  (Utilities|Array|Resize (Variables|Default|GetAll%20Enemies) (Variables|Properties|GetSpawn%20Limit)))

(event EventEndPlay
  (params (EndPlayReason :type EEndPlayReason%20Enum :default "Destroyed"))
  (for _array_element (Variables|Default|GetAll%20Enemies)
    (Utilities|IsValid _array_element
      (:Is%20Valid
        (EventDispatchers|UnbindallEventsfromOnEnemyDeactivated _array_element)))))

(fn ConstructionScript
  (bind _returnvalue (Transformation|GetActorLocation))
  (bind (_x _y _z) (Math|Vector|BreakVector _returnvalue))
  (Transformation|SetActorLocation (Math|Vector|MakeVector 0.0 0.0 (Variables|Default|GetLocation%20Z)) false false)
  (Rendering|Debug|FlushPersistentDebugLines)
  (Rendering|Debug|DrawDebugBox (Math|Vector|MakeVector _x _y (+ _z (.Z (Math|Vector|BreakVector (Variables|Properties|GetSpawning%20Area))))) (Variables|Properties|GetSpawning%20Area) "(R=0.208333,G=0.208333,B=0.208333,A=1.000000)" "0, 0, 0" 3e+01 5.0))

(fn GetRandomLocationInsideArea
  (bind _returnvalue (Transformation|GetActorLocation))
  (bind _spawning_area (Variables|Properties|GetSpawning%20Area))
  (bind (_x _y) (Math|Vector|BreakVector _spawning_area))
  (bind (_x_2 _y_2 _z) (Math|Vector|BreakVector _returnvalue))
  (bind _returnvalue_2 (/ _x 2.0))
  (bind _returnvalue_3 (/ _y 2.0))
  (return (Math|Vector|MakeVector (Math|Random|RandomFloatinRange (- _x_2 _returnvalue_2) (+ _x_2 _returnvalue_2)) (Math|Random|RandomFloatinRange (- _y_2 _returnvalue_3) (+ _y_2 _returnvalue_3)) _z)))