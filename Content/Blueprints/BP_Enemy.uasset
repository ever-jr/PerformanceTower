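; BP_Enemy is a reusable enemy that walks toward the BP_Canon found at BeginPlay and damages it on arrival.
; Each tick it yaws to face the cannon and steps forward by StepDistance per second, calling HitTarget once within StepDistance of it.
; Instead of being destroyed, it toggles tick and root visibility through ActivateActor and DeactiveActor, and HitTarget broadcasts OnEnemyDeactivated, which suits pooling.
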(event Custom|Hit%20Target
  (bind _canon_ref (Variables|Default|GetCanon%20Ref)
    (:then
      (Default|DealDamage _canon_ref self (Variables|Default|GetDamage))
      (Development|PrintString "Hit canon"))
    (:else
      _))
  (CallFunction|DeactiveActor)
  (Default|CallOnEnemyDeactivated self))

(event Custom|Deactive%20Actor
  (Actor|Tick|SetActorTickEnabled false)
  (Rendering|SetVisibility (Variables|Default|GetDefaultSceneRoot) false false))

(event Custom|Activate%20Actor
  (params (Location :type Vector))
  (Transformation|SetActorLocation Location false false)
  (Actor|Tick|SetActorTickEnabled true)
  (Rendering|SetVisibility (Variables|Default|GetDefaultSceneRoot) true false))

(event EventBeginPlay
  (bind _returnvalue (Actor|GetActorOfClass "/Game/Blueprints/BP_Canon.BP_Canon_C"))
  (Variables|Default|SetCanon%20Ref _returnvalue))

(event EventTick
  (params (DeltaSeconds :type Float%20%28single-precision%29))
  (bind _canon_ref (Variables|Default|GetCanon%20Ref)
    (:then
      (Transformation|SetActorRotation (Math|Rotator|MakeRotator 0.0 0.0 (.Yaw (Math|Rotator|BreakRotator (Math|Rotator|FindLookatRotation (Transformation|GetActorLocation) (Transformation|GetActorLocation _canon_ref))))))
      (Transformation|SetActorLocation (+ (* (Transformation|GetActorForwardVector) (* (Variables|Default|GetStep%20Distance) DeltaSeconds)) (Transformation|GetActorLocation)) false false)
      (if (<= (Transformation|GetDistanceTo self (Variables|Default|GetCanon%20Ref)) (Variables|Default|GetStep%20Distance))
        (CallFunction|HitTarget)))
    (:else)))

(fn ConstructionScript)