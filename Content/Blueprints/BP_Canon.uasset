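; BP_Canon is a cannon Blueprint with a health value that can take damage.
; Its DealDamage function subtracts the damage from Health, clamps the result at zero and prints the remaining health as debug text.
; BeginPlay and the construction script are empty, and reaching zero health triggers nothing further.
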(event EventBeginPlay)

(fn ConstructionScript)

(fn DealDamage
  (params (Damage%20Source :type Actor%20Object%20Reference) (Damage :type Float%20%28double-precision%29))
  (LocalVariables|SetNew%20Health%20%28Local%29 (- (Variables|Default|GetHealth) Damage))
  (if (> (LocalVariables|GetNew%20Health%20%28Local%29) 0.0)
    _
    (else
      (LocalVariables|SetNew%20Health%20%28Local%29 0.0)))
  (Variables|Default|SetHealth (LocalVariables|GetNew%20Health%20%28Local%29))
  (Development|PrintText (Utilities|Text|FormatText "Canon health: {Health}" (Variables|Default|GetHealth))))